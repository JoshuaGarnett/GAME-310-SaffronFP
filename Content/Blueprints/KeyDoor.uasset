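; KeyDoor is a door actor that unlocks when the third-person character touches its trigger box while holding a key of the required color.
; On overlap it checks that color's slot in the character's KeyAmounts array, opens the door, deducts one key and prints the remaining amounts.
; OpenDoor sets an Unlocked flag, and Tick then swings the door open by incremental yaw rotation per frame until it reaches a quarter turn.
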(event `self.ReceiveTick`
  (params (DeltaSeconds :type "Float (single-precision)"))
  (if (== (`self.Unlocked`) true)
    (if (< (`self.RotateAmount`) 90.0)
      (`SceneComponent.K2_AddLocalRotation` (`self.Door`) (struct :`Yaw` -1.0) false false)
      (set `self.RotateAmount` (+ (`self.RotateAmount`) 1.0)))))

(event `self.Box.OnComponentBeginOverlap`
  (params (OverlappedComponent :type "PrimitiveComponent Object Reference") (OtherActor :type "Actor Object Reference") (OtherComp :type "PrimitiveComponent Object Reference") (OtherBodyIndex :type Integer) (bFromSweep :type Boolean) (SweepResult :type "HitResult Structure (by ref)"))
  (bind _keycolorrequired (`self.KeyColorRequired`))
  (bind _asbp_third_person_character (cast `/Game/ThirdPerson/Blueprints/BP_ThirdPersonCharacter` OtherActor)
    (:`then`
      (bind _keyamounts (`/Game/ThirdPerson/Blueprints/BP_ThirdPersonCharacter.KeyAmounts` _asbp_third_person_character))
      (bind _output (`|GetArrayItem` _keyamounts _keycolorrequired))
      (if (>= _output 1.0)
        (`KismetSystemLibrary.PrintString` "Door Opened")
        (`self.OpenDoor`)
        (`KismetArrayLibrary.Array_Set` _keyamounts _keycolorrequired (- _output 1.0))
        (`/Game/ThirdPerson/Blueprints/BP_ThirdPersonCharacter.PrintKeyAmounts` _asbp_third_person_character)
        (else
          (`KismetSystemLibrary.PrintString` "DoorLocked"))))
    (:`CastFailed`
      (`KismetSystemLibrary.PrintString` "Cast Failed"))))

(fn `OpenDoor`
  (`KismetSystemLibrary.PrintString` "Opening Door")
  (set `self.Unlocked` true))

(fn `UserConstructionScript`)