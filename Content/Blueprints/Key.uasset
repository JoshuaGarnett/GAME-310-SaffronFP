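; Key is a colored pickup actor that the third-person player character collects by touching its Box component.
; On overlap it casts to BP_ThirdPersonCharacter, increments that character's KeyAmounts entry indexed by the key's Color, calls PrintKeyAmounts, then destroys itself.
; Overlaps from any other actor only print a "Not Player" debug string.
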(event `self.Box.OnComponentBeginOverlap`
  (params (OverlappedComponent :type "PrimitiveComponent Object Reference") (OtherActor :type "Actor Object Reference") (OtherComp :type "PrimitiveComponent Object Reference") (OtherBodyIndex :type Integer) (bFromSweep :type Boolean) (SweepResult :type "HitResult Structure (by ref)"))
  (bind _asbp_third_person_character (cast `/Game/ThirdPerson/Blueprints/BP_ThirdPersonCharacter` OtherActor)
    (:`then`
      (`KismetArrayLibrary.Array_Set` (`/Game/ThirdPerson/Blueprints/BP_ThirdPersonCharacter.KeyAmounts` _asbp_third_person_character) (`self.Color`) (+ (`|GetArrayItem` (`/Game/ThirdPerson/Blueprints/BP_ThirdPersonCharacter.KeyAmounts` _asbp_third_person_character) (`self.Color`)) 1.0))
      (`/Game/ThirdPerson/Blueprints/BP_ThirdPersonCharacter.PrintKeyAmounts` _asbp_third_person_character)
      (`self.K2_DestroyActor`))
    (:`CastFailed`
      (`KismetSystemLibrary.PrintString` "Not Player"))))

(fn `UserConstructionScript`)