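; Draggable object actor that follows the third-person player character while that character is grabbing.
; A Collision overlap casts to BP_ThirdPersonCharacter, stores the reference and sets a collided flag, which is never cleared here.
; While the flag and the character's Grabbing state are true, Tick places the Cube at a horizontal Offset along the character's forward vector, matching its rotation and keeping its own scale.
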(event `self.ReceiveTick`
  (params (DeltaSeconds :type "Float (single-precision)"))
  (bind _tpc (`self.TPC`))
  (bind _offset (`self.Offset`))
  (bind _cube (`self.Cube`))
  (bind (_returnvalue_location _returnvalue_rotation) (`KismetMathLibrary.BreakTransform` (`self.GetTransform` (`self.TPC`))))
  (if (`self.PlayerCollided`)
    (if (!= _tpc null)
      (if (`/Game/ThirdPerson/Blueprints/BP_ThirdPersonCharacter.Grabbing` _tpc)
        (`KismetSystemLibrary.PrintString` "Grabbing")
        (`SceneComponent.K2_SetWorldTransform` _cube (`KismetMathLibrary.MakeTransform` (+ _returnvalue_location (* (`KismetMathLibrary.GetForwardVector` _returnvalue_rotation) (`KismetMathLibrary.MakeVector` _offset _offset))) (* _returnvalue_rotation 1.0) (`SceneComponent.K2_GetComponentScale` _cube)) false false)))))

(event `self.Collision.OnComponentBeginOverlap`
  (params (OverlappedComponent :type "PrimitiveComponent Object Reference") (OtherActor :type "Actor Object Reference") (OtherComp :type "PrimitiveComponent Object Reference") (OtherBodyIndex :type Integer) (bFromSweep :type Boolean) (SweepResult :type "HitResult Structure (by ref)"))
  (bind _asbp_third_person_character (cast `/Game/ThirdPerson/Blueprints/BP_ThirdPersonCharacter` OtherActor)
    (:`then`
      (set `self.TPC` _asbp_third_person_character)
      (set `self.PlayerCollided` true)
      (`KismetSystemLibrary.PrintString` "Collided"))
    (:`CastFailed`
      (`KismetSystemLibrary.PrintString` "Cast Failed"))))

(fn `UserConstructionScript`)